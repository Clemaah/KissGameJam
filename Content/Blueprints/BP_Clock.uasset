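; BP_Clock is an analog clock actor whose hands show the in-game time.
; On BeginPlay it limits its scene capture to its own components and binds UpdateHands to BP_GameMode's hour-updated event.
; Each update sets the roll of the hour and minute hands from the two components of the current time, with an angular offset on the hour hand.
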(event `self.ReceiveBeginPlay`
  (`SceneCaptureComponent.ShowOnlyActorComponents` (`self.SceneCaptureComponent2D`) self false)
  (bind _asbp_game_mode (cast `/Game/Blueprints/System/BP_GameMode` (`GameplayStatics.GetGameMode`)))
  (add `/Game/Blueprints/System/BP_GameMode.OnHourUpdated` _asbp_game_mode (delegate `UpdateHands`)))

(event `UpdateHands`
  (params (CurrentHour :type "Vector2D Structure (by ref)"))
  (`SceneComponent.K2_SetRelativeRotation` (`self.HourHand`) (`KismetMathLibrary.MakeRotator` (+ (* CurrentHour_X 30.0) 90.0)) false false)
  (`SceneComponent.K2_SetRelativeRotation` (`self.MinuteHand`) (`KismetMathLibrary.MakeRotator` (* CurrentHour_Y 6.0)) false false))

(fn `UserConstructionScript`)