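; Interactable lamp that the player can break, killing its spotlights and lighting zone while making noise.
; Overlapping the interaction zone enables interaction and an outline overlay, checked on Tick.
; Timer events show or hide a world widget with a Timeline-driven progress bar, pitched from the player camera.
; Interact swaps materials, reports a noise event, plays break VFX and sound, and animates a post-process noise ripple through a parameter collection.
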(event `self.ReceiveTick`
  (params (DeltaSeconds :type "Float (single-precision)"))
  (bind _lamp (`self.Lamp`))
  (bind _asbp_character (cast `/Game/Blueprints/System/BP_Character` (`GameplayStatics.GetPlayerCharacter` 0)))
  (if (`PrimitiveComponent.IsOverlappingActor` (`self.InteractionZone`) _asbp_character)
    (`MeshComponent.SetOverlayMaterial` _lamp "/Game/Materials/outlinesTriggerable/M_outlineLamp.M_outlineLamp")
    (`MeshComponent.SetOverlayMaterial` (`self.Glass1`) "/Game/Materials/outlinesTriggerable/M_outlineLamp.M_outlineLamp")
    (`MeshComponent.SetOverlayMaterial` (`self.Glass2`) "/Game/Materials/outlinesTriggerable/M_outlineLamp.M_outlineLamp")
    (else
      (`MeshComponent.SetOverlayMaterial` _lamp "/Game/Materials/outlinesTriggerable/M_empty.M_empty")
      (`MeshComponent.SetOverlayMaterial` (`self.Glass1`) "/Game/Materials/outlinesTriggerable/M_empty.M_empty")
      (`MeshComponent.SetOverlayMaterial` (`self.Glass2`) "/Game/Materials/outlinesTriggerable/M_empty.M_empty"))))

(event `/Game/Blueprints/BPI_Interact.StartTimer`
  (bind _asbp_character (cast `/Game/Blueprints/System/BP_Character` (`GameplayStatics.GetPlayerCharacter` 0)))
  (bind (_returnvalue_roll _returnvalue_pitch) (`KismetMathLibrary.BreakRotator` (`SceneComponent.K2_GetComponentRotation` (`/Game/Blueprints/System/BP_Character.Camera` _asbp_character))))
  (`SceneComponent.K2_SetWorldRotation` (`self.Widget`) (`KismetMathLibrary.MakeRotator` 0.0 (+ _returnvalue_pitch 160.0) 180.0) false false)
  (`Widget.SetVisibility` (`self.3DWidget`) "Visible")
  (bind (_direction _pbvalue) (`Timeline|Timeline`)
    (:`Update`
      (`ProgressBar.SetPercent` (`/Game/UI/WBP_InGame.ProgressBar` (`self.3DWidget`)) _pbvalue))))

(event `/Game/Blueprints/BPI_Interact.EndTimer`
  (`Widget.SetVisibility` (`self.3DWidget`) "Hidden"))

(event `self.ReceiveBeginPlay`
  (bind _widget (`self.Widget`))
  (bind _returnvalue (`|GenericCreateObject` _widget "/Game/UI/WBP_InGame.WBP_InGame_C"))
  (bind _output_get (set `self.3DWidget` _returnvalue))
  (`WidgetComponent.SetWidget` _widget _output_get)
  (`Widget.SetVisibility` (`self.3DWidget`) "Hidden"))

(event `/Game/Blueprints/BPI_Interact.Interact`
  ;[0.06511 0.1006 0.1177] Destroys light
  (`PrimitiveComponent.SetCollisionEnabled` (`self.InteractionZone`) "NoCollision")
  (`PrimitiveComponent.SetMaterial` (`self.Lamp`) 0 "/Game/Materials/metal.metal")
  (`PrimitiveComponent.SetMaterial` (`self.Glass1`) 0 "/Game/Materials/metal.metal")
  (`PrimitiveComponent.SetMaterial` (`self.Glass2`) 0 "/Game/Materials/metal.metal")
  (`AISense_Hearing.ReportNoiseEvent` (+ (`self.K2_GetActorLocation`) (* (`KismetMathLibrary.Vector_Backward`) 200)) 1.0 self 2000.0)
  (`PrimitiveComponent.SetCollisionEnabled` (`self.LightingZone`) "NoCollision")
  (`ActorComponent.Activate` (`self.VFX_lampBreak`) false)
  (`ActorComponent.Activate` (`self.VFX_noiseRipple`) false)
  (`GameplayStatics.PlaySound2D` "/Game/Audio/Sounds/Effects/Lamps/Lightbulb_Break_2B_Cue.Lightbulb_Break_2B_Cue" 1.0 1.0 0.0 null null)
  (`ActorComponent.K2_DestroyComponent` (`self.SpotLight1`))
  (`ActorComponent.K2_DestroyComponent` (`self.SpotLight`))
  (bind (_direction _noiseripple) (`Timeline|TimelineNoiseRipple` :!via `PlayFromStart`)
    (:`Update`
      (`KismetMaterialLibrary.SetScalarParameterValue` "/Game/Materials/postProcess/MPC_PostProcess.MPC_PostProcess" "noiseRipple" _noiseripple))))

(fn `GetInteractionDelay`
  (returns (Delay :type "Float (double-precision)"))
  (return (`self.InteractionDelay`)))

(fn `IsInteractable`
  (returns (IsInteractable :type Boolean))
  (return (`PrimitiveComponent.IsOverlappingActor` (`self.InteractionZone`) (`GameplayStatics.GetPlayerCharacter` 0))))

(fn `UserConstructionScript`)