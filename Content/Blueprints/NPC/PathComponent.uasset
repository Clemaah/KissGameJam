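; NPC path component that builds a random list of path points from the BP_PathPoint actors in the level.
; On BeginPlay it loops a random number of times, from a minimum of four up to the point count, adding random picks to PathPoints.
; Each pass removes a separately rolled index from the available pool, so points can repeat.
; OnPathInitializationFinished is called inside the loop, on every pass.
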(event `self.ReceiveBeginPlay`
  (bind (_outitem _outindex) (`KismetArrayLibrary.Array_Random` (`self.AvailablePoints`)))
  (bind _outactors (`GameplayStatics.GetAllActorsOfClass` "/Game/Blueprints/NPC/BP_PathPoint.BP_PathPoint_C"))
  (bind _output_get (set `self.AvailablePoints` _outactors))
  (for _ (range (+ (`KismetMathLibrary.RandomIntegerInRange` 4 (`KismetArrayLibrary.Array_Length` _output_get)) 1))
    (`KismetArrayLibrary.Array_Add` (`self.PathPoints`) _outitem)
    (`KismetArrayLibrary.Array_Remove` (`self.AvailablePoints`) _outindex)
    (`self.OnPathInitializationFinished`)))