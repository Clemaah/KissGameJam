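; BP_Cop is a cop NPC that ends the game when the player character touches it.
; Its Killzone overlap casts to BP_Character, then pauses the game, disables Killzone collision and shows the UI_ending widget.
; Each Tick, ToggleFootTrailVFX turns the footstep trail effect on above a speed threshold and deactivates and resets it below, acting only on state changes.
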(event `self.ReceiveBeginPlay`
  (bind _vfx_footsteptrail (`self.VFX_footstepTrail`))
  (`ActorComponent.Deactivate` _vfx_footsteptrail)
  (`NiagaraComponent.ResetSystem` _vfx_footsteptrail))

(event `self.killzone.OnComponentBeginOverlap`
  (params (OverlappedComponent :type "PrimitiveComponent Object Reference") (OtherActor :type "Actor Object Reference") (OtherComp :type "PrimitiveComponent Object Reference") (OtherBodyIndex :type Integer) (bFromSweep :type Boolean) (SweepResult :type "HitResult Structure (by ref)"))
  (bind _asbp_top_down_character (cast `/Game/Blueprints/System/BP_Character` OtherActor))
  (`/Engine/EditorBlueprintResources/StandardMacros.IsValid` _asbp_top_down_character
    (:`Is Valid`
      (`GameplayStatics.SetGamePaused` true)
      (`PrimitiveComponent.SetCollisionEnabled` (`self.killzone`) "NoCollision")
      (bind _returnvalue (`|CreateWidget` "/Game/UI/UI_ending.UI_ending_C"))
      (`UserWidget.AddToViewport` _returnvalue 0))))

(event `self.ReceiveTick`
  (params (DeltaSeconds :type "Float (single-precision)"))
  (if (`ActorComponent.IsActive` (`self.VFX_footstepTrail`))
    (if (< (`KismetMathLibrary.VSize` (`self.GetVelocity`)) 400.0)
      (`ActorComponent.Deactivate` (`self.VFX_footstepTrail`))
      (`NiagaraComponent.ResetSystem` (`self.VFX_footstepTrail`)))
    (elif (>= (`KismetMathLibrary.VSize` (`self.GetVelocity`)) 400.0)
      (`ActorComponent.Activate` (`self.VFX_footstepTrail`) false))))

(fn `UserConstructionScript`)