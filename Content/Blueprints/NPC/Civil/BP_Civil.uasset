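; Civilian NPC that the player can kill through a timed interaction, with a random male or female mesh, animation and scream set at spawn.
; A 3D progress widget shows the interaction timer, while Tick outlines the civilian in range and toggles a speed-based footstep trail.
; Interact ragdolls it with blood VFX and a spreading decal, calls OnCivilKilled, then copies the pose to a PoseableMesh that sinks away.
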(event `self.ReceiveBeginPlay`
  (bind _widget (`self.Widget`))
  (bind _returnvalue (`|GenericCreateObject` _widget "/Game/UI/WBP_InGame.WBP_InGame_C"))
  (bind _output_get (set `self.3DWidget` _returnvalue))
  (`WidgetComponent.SetWidget` _widget _output_get)
  (`Widget.SetVisibility` (`self.3DWidget`) "Hidden")
  (switch `int` (`KismetMathLibrary.RandomIntegerInRange` 0 1)
    (:`Default`
      (`SkeletalMeshComponent.SetSkeletalMeshAsset` (`self.Mesh`) "/Game/Characters/PNJ/Puka/Idle/IdlePuka.IdlePuka")
      (`SkeletalMeshComponent.SetAnimInstanceClass` (`self.Mesh`) "/Game/Characters/PNJ/Puka/Walk/ABP_PUKA.ABP_PUKA_C")
      (`AudioComponent.SetSound` (`self.ScreamAfraidAudio`) "/Game/Audio/Sounds/Screams/WomenScreamAfraidCue.WomenScreamAfraidCue")
      (`AudioComponent.SetSound` (`self.ScreamDeathAudio`) "/Game/Audio/Sounds/Screams/WomenScreamDeathCue.WomenScreamDeathCue"))
    (:`0`
      (`SkeletalMeshComponent.SetSkeletalMeshAsset` (`self.Mesh`) "/Game/Characters/PNJ/Robert/Idle/IdleRobert.IdleRobert")
      (`SkeletalMeshComponent.SetAnimInstanceClass` (`self.Mesh`) "/Game/Characters/PNJ/Robert/Idle/ABP_Robert.ABP_Robert_C")
      (`AudioComponent.SetSound` (`self.ScreamAfraidAudio`) "/Game/Audio/Sounds/Screams/MenScreamAfraidCue.MenScreamAfraidCue")
      (`AudioComponent.SetSound` (`self.ScreamDeathAudio`) "/Game/Audio/Sounds/Screams/MenScreamDeathCue.MenScreamDeathCue")))
  (`SkinnedMeshComponent.SetSkinnedAssetAndUpdate` (`self.PoseableMesh`) (`SkinnedMeshComponent.GetSkinnedAsset` (`self.Mesh`)) true))

(event `self.Interact`
  (`AudioComponent.Play` (`self.ScreamDeathAudio`) 0.0)
  (set `self.IsDead` true)
  (`self.DetachFromControllerPendingDestroy`)
  (`SceneComponent.K2_SetWorldRotation` (`self.VFX_slashBlood`) (`KismetMathLibrary.Conv_VectorToRotator` (- (`SceneComponent.K2_GetComponentLocation` (`self.Mesh`)) (`SceneComponent.K2_GetComponentLocation` (`Actor.RootComponent` (`GameplayStatics.GetPlayerCharacter` 0))))) false false)
  (`ActorComponent.Activate` (`self.VFX_slashBlood`) false)
  (`PrimitiveComponent.SetSimulatePhysics` (`self.Mesh`) true)
  (`PrimitiveComponent.SetCollisionProfileName` (`self.Mesh`) "Ragdoll" true)
  (`PrimitiveComponent.SetCollisionEnabled` (`self.InteractionZone`) "NoCollision")
  (`PrimitiveComponent.SetCollisionEnabled` (`self.CapsuleComponent`) "NoCollision")
  (`SceneComponent.SetHiddenInGame` (`self.Decal`) false false)
  (bind _returnvalue (`DecalComponent.CreateDynamicMaterialInstance` (`self.Decal`)))
  (bind (_direction _spread) (`Timeline|TimelineSpread`)
    (:`Update`
      (`MaterialInstanceDynamic.SetScalarParameterValue` _returnvalue "spread" _spread))
    (:`Finished`
      (`self.OnCivilKilled`)
      (for _array_element (`SceneComponent.GetAllSocketNames` (`self.Mesh`))
        (`PoseableMeshComponent.SetBoneTransformByName` (`self.PoseableMesh`) _array_element (`SceneComponent.GetSocketTransform` (`self.Mesh`) _array_element "RTS_World") "WorldSpace"))
      (`KismetSystemLibrary.Delay` 0.1)
      (`PrimitiveComponent.SetSimulatePhysics` (`self.Mesh`) false)
      (`SceneComponent.SetVisibility` (`self.Mesh`) false false)
      (`SceneComponent.SetVisibility` (`self.PoseableMesh`) true false)
      (bind (_direction_2 _alpha) (`Timeline|TimelineDisparition` :!via `PlayFromStart`)
        (:`Update`
          (`SceneComponent.K2_SetRelativeLocation` (`self.PoseableMesh`) (`KismetMathLibrary.MakeVector` 0.0 0.0 (+ (* _alpha -300.0) -80.0)) false false))
        (:`Finished`
          (`PrimitiveComponent.SetCollisionEnabled` (`self.CapsuleComponent`) "NoCollision"))))))

(event `self.StartTimer`
  (bind _asbp_character (cast `/Game/Blueprints/System/BP_Character` (`GameplayStatics.GetPlayerCharacter` 0)))
  (bind (_returnvalue_roll _returnvalue_pitch) (`KismetMathLibrary.BreakRotator` (`SceneComponent.K2_GetComponentRotation` (`/Game/Blueprints/System/BP_Character.Camera` _asbp_character))))
  (`SceneComponent.K2_SetWorldRotation` (`self.Widget`) (`KismetMathLibrary.MakeRotator` 0.0 (+ _returnvalue_pitch 160.0) 180.0) false false)
  (`Widget.SetVisibility` (`self.3DWidget`) "Visible")
  (bind (_direction _pbvalue) (`Timeline|Timeline` :!via `PlayFromStart`)
    (:`Update`
      (`ProgressBar.SetPercent` (`/Game/UI/WBP_InGame.ProgressBar` (`self.3DWidget`)) _pbvalue))))

(event `self.EndTimer`
  (`Widget.SetVisibility` (`self.3DWidget`) "Hidden"))

(event `self.ReceiveTick`
  (params (DeltaSeconds :type "Float (single-precision)"))
  (if (`ActorComponent.IsActive` (`self.VFX_footstepTrail`))
    (if (< (`KismetMathLibrary.VSize` (`self.GetVelocity`)) 400.0)
      (`ActorComponent.Deactivate` (`self.VFX_footstepTrail`))
      (`NiagaraComponent.ResetSystem` (`self.VFX_footstepTrail`))
      (bind _asbp_character (cast `/Game/Blueprints/System/BP_Character` (`GameplayStatics.GetPlayerCharacter` 0) :!label _label))
      (if (`PrimitiveComponent.IsOverlappingActor` (`self.InteractionZone`) _asbp_character)
        (`MeshComponent.SetOverlayMaterial` (`self.Mesh`) "/Game/Materials/outlinesTriggerable/M_outlineKill.M_outlineKill")
        (else
          (`MeshComponent.SetOverlayMaterial` (`self.Mesh`) "/Game/Materials/outlinesTriggerable/M_empty.M_empty"))))
    (elif (>= (`KismetMathLibrary.VSize` (`self.GetVelocity`)) 400.0)
      (`ActorComponent.Activate` (`self.VFX_footstepTrail`) false)
      (goto _label))))

(fn `GetInteractionDelay`
  (returns (Delay :type "Float (double-precision)"))
  (return (`self.InteractionDelay`)))

(fn `IsInteractable`
  (returns (IsInteractable :type Boolean))
  (return true))

(fn `UserConstructionScript`)