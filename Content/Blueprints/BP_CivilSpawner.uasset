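; BP_CivilSpawner populates the level with civilian and cop NPCs and adds a new civilian whenever the player character signals a kill.
; After a short delay on BeginPlay, it reads the current level's NPC counts from BP_GameInstance and spawns that many at random points from an all-matching EQS query.
; Each kill reruns the same player-centered query in random-best-5% mode to place one BP_Civil; cops are never respawned here.
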(event `self.ReceiveBeginPlay`
  (`KismetSystemLibrary.Delay` 0.2)
  (bind _asbp_game_instance (cast `/Game/Blueprints/System/BP_GameInstance` (`GameplayStatics.GetGameInstance`)))
  (set `self.CurrentLevel` (`/Game/Blueprints/System/BP_GameInstance.GetCurrentLevel` _asbp_game_instance))
  (bind _asbp_top_down_character (cast `/Game/Blueprints/System/BP_Character` (`GameplayStatics.GetPlayerCharacter` 0)))
  (add `/Game/Blueprints/System/BP_Character.OnNewKill` _asbp_top_down_character (delegate `SpawnNPC`))
  (`self.InitialSpawn`))

(event `SpawnNPC`
  ;[1 1 1] Respawn
  (bind _returnvalue (`EnvQueryManager.RunEQSQuery` "/Game/Blueprints/NPC/GetSpawnLocation.GetSpawnLocation" (`GameplayStatics.GetPlayerCharacter` 0) "RandomBest5Pct"))
  (add `EnvQueryInstanceBlueprintWrapper.OnQueryFinishedEvent` _returnvalue (delegate `OnQueryFinishedEventCop`)))

(event `OnQueryFinishedEventCop`
  (params (QueryInstance :type "EnvQueryInstanceBlueprintWrapper Object Reference") (QueryStatus :type "EEnvQueryStatus Enum" :default "Processing"))
  ;[1 1 1] Respawn
  (bind _resultlocations (`EnvQueryInstanceBlueprintWrapper.GetQueryResultsAsLocations` QueryInstance))
  (`|SpawnActorFromClass` "/Game/Blueprints/NPC/Civil/BP_Civil.BP_Civil_C" (`KismetMathLibrary.MakeTransform` (`|GetArrayItem` _resultlocations)) "Undefined" "MultiplyWithRoot" null null))

(event `InitialSpawn`
  ;[1 1 1] InitialSpawn
  (bind _returnvalue (`EnvQueryManager.RunEQSQuery` "/Game/Blueprints/NPC/GetSpawnLocation.GetSpawnLocation" (`GameplayStatics.GetPlayerCharacter` 0) "AllMatching"))
  (add `EnvQueryInstanceBlueprintWrapper.OnQueryFinishedEvent` _returnvalue (delegate `OnQueryFinishedEventSpawn`)))

(event `OnQueryFinishedEventSpawn`
  (params (QueryInstance :type "EnvQueryInstanceBlueprintWrapper Object Reference") (QueryStatus :type "EEnvQueryStatus Enum" :default "Processing"))
  (bind _currentlevel_nbcops (break `/Game/Blueprints/S_Level` (`self.CurrentLevel`)))
  (bind (_currentlevel_nbcops_2 _currentlevel_nbcivils) (break `/Game/Blueprints/S_Level` (`self.CurrentLevel`)))
  ;[1 1 1] InitialSpawn
  (bind _resultlocations (`EnvQueryInstanceBlueprintWrapper.GetQueryResultsAsLocations` QueryInstance))
  (for _ (range 1 (+ _currentlevel_nbcivils 1))
    (bind _outitem (`KismetArrayLibrary.Array_Random` _resultlocations))
    (`|SpawnActorFromClass` "/Game/Blueprints/NPC/Civil/BP_Civil.BP_Civil_C" (`KismetMathLibrary.MakeTransform` _outitem) "AdjustIfPossibleButAlwaysSpawn" "MultiplyWithRoot" null null))
  (for _ (range 1 (+ _currentlevel_nbcops 1))
    (`|SpawnActorFromClass` "/Game/Blueprints/NPC/Cop/BP_Cop.BP_Cop_C" (`KismetMathLibrary.MakeTransform` _outitem) "AdjustIfPossibleButAlwaysSpawn" "MultiplyWithRoot" null null)))

(fn `UserConstructionScript`)