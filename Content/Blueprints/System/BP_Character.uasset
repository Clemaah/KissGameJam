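; Player character for a timed night stealth game, with movement, sprint, pause and delayed interactions, including killing civilians.
; Interacting picks a nearby BPI_Interact actor and locks input until a timer completes.
; Overlapping BP_Light actors determine whether the player is hidden, driving visibility notifications and a post-process ambiance timeline.
; Tick tilts the spring arm when the camera trace is blocked and toggles speed-based footstep VFX, while a countdown ends the night.
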(event `self.ReceiveBeginPlay`
  ;[0.06511 0.1006 0.1177] Initialize controls
  (`parent.ReceiveBeginPlay`)
  (`EnhancedInputSubsystemInterface.AddMappingContext` (pcsubsystem `EnhancedInputLocalPlayerSubsystem` (`GameplayStatics.GetPlayerController` 0)) "/Game/Input/IMC_Default.IMC_Default" 0 (struct))
  (`KismetSystemLibrary.K2_SetTimer` null "ChangeCountdown" 1.0 true)
  (`KismetSystemLibrary.Delay` 0.5)
  (`self.UpdateVisibilityState`))

(event `EnhancedInput|/Game/Input/Actions/INP_Move`
  (params (ActionValue :type "Vector2D Structure") (ElapsedSeconds :type "Float (double-precision)") (TriggeredSeconds :type "Float (double-precision)") (InputAction :type "InputAction Object Reference" :default "/Game/Input/Actions/INP_Move.INP_Move"))
  ;[0.06511 0.1006 0.1177] Character movements
  (:`Triggered`
    (`self.AddMovementInput` (0.0 1.0 0.0) ActionValue_X) ; Horizontal move
    (`self.AddMovementInput` (1.0 0.0 0.0) ActionValue_Y) ; Vertical move
  ))

(event `EnhancedInput|/Game/Input/Actions/INP_Interact`
  (params (ActionValue :type Boolean) (ElapsedSeconds :type "Float (double-precision)") (TriggeredSeconds :type "Float (double-precision)") (InputAction :type "InputAction Object Reference" :default "/Game/Input/Actions/INP_Interact.INP_Interact"))
  ;[0.06511 0.1006 0.1177] Interact
  (:`Started`
    (`self.InteractBehaviour`)))

(event `Interaction`
  (bind _elementtointeract (`self.ElementToInteract`))
  ;[0.06511 0.1006 0.1177] Interact
  (`/Game/Blueprints/BPI_Interact.EndTimer` _elementtointeract)
  (`/Game/Blueprints/BPI_Interact.Interact` _elementtointeract)
  (`self.EnableInput` (`GameplayStatics.GetPlayerController` 0))
  (cast `/Game/Blueprints/NPC/Civil/BP_Civil` (`self.ElementToInteract`))
  (`GameplayStatics.PlayWorldCameraShake` "/Game/Blueprints/BP_CameraShake.BP_CameraShake_C" (`SceneComponent.K2_GetComponentLocation` (`self.Camera`)) 0.0 100.0)
  (`self.OnNewKill`)
  (`GameplayStatics.PlaySound2D` "/Game/Audio/Sound/Slash/slash.slash" 1.0 1.0 0.0 null null)
  (set `self.isKilling?` true)
  (`KismetSystemLibrary.Delay` 0.5)
  (set `self.isKilling?` false))

(event `EnhancedInput|/Game/Input/Actions/INP_Pause`
  (params (ActionValue :type Boolean) (ElapsedSeconds :type "Float (double-precision)") (TriggeredSeconds :type "Float (double-precision)") (InputAction :type "InputAction Object Reference" :default "/Game/Input/Actions/INP_Pause.INP_Pause"))
  ;[1 1 1] Pause Menu
  (:`Triggered`
    (if (`GameplayStatics.IsGamePaused`)
      (`Widget.RemoveFromParent` (stale _returnvalue))
      (`GameplayStatics.SetGamePaused` false)
      (else
        (bind _returnvalue (`|CreateWidget` "/Game/UI/UI_Paused.UI_Paused_C"))
        (`UserWidget.AddToViewport` _returnvalue 0)
        (`GameplayStatics.SetGamePaused` true)))))

(event `EnhancedInput|/Game/Input/Actions/INP_Sprint`
  (params (ActionValue :type Boolean) (ElapsedSeconds :type "Float (double-precision)") (TriggeredSeconds :type "Float (double-precision)") (InputAction :type "InputAction Object Reference" :default "/Game/Input/Actions/INP_Sprint.INP_Sprint"))
  (bind _charactermovement (`self.CharacterMovement`))
  ;[0.06511 0.1006 0.1177] Sprint
  (:`Started`
    (set `CharacterMovementComponent.MaxWalkSpeed` (`self.SprintSpeed`) _charactermovement))
  (:`Completed`
    (set `CharacterMovementComponent.MaxWalkSpeed` (`self.WalkSpeed`) _charactermovement)))

(event `self.ReceiveActorBeginOverlap`
  (params (OtherActor :type "Actor Object Reference"))
  ;[0.06511 0.1006 0.1177] Zone type management
  (`self.UpdateVisibilityState` :!label _label))

(event `self.ReceiveActorEndOverlap`
  (params (OtherActor :type "Actor Object Reference"))
  ;[0.06511 0.1006 0.1177] Zone type management
  (goto _label))

(event `self.ReceiveTick`
  (params (DeltaSeconds :type "Float (single-precision)"))
  ;[0.06511 0.1006 0.1177] Camera orientation
  (if (`ActorComponent.IsActive` (`self.VFX_footstepTrail`))
    (if (< (`KismetMathLibrary.VSize` (`self.GetVelocity`)) 400.0)
      (`ActorComponent.Deactivate` (`self.VFX_footstepTrail`))
      (`NiagaraComponent.ResetSystem` (`self.VFX_footstepTrail`))
      (bind _outhit (`KismetSystemLibrary.LineTraceSingle` (`SceneComponent.K2_GetComponentLocation` (`self.CameraLocation`)) (`SceneComponent.K2_GetComponentLocation` (`self.Scene`)) "TraceTypeQuery2" :!label _label_2))
      (if (`GameplayStatics.BreakHitResult` _outhit)
        (bind (_direction _rotation) (`Timeline|Timeline` :!label _label_3)
          (:`Update`
            (`SceneComponent.K2_SetRelativeRotation` (`self.SpringArm`) (`KismetMathLibrary.MakeRotator` 0.0 _rotation) false false)))
        (else
          (goto _label_3 :!via `Reverse`))))
    (elif (>= (`KismetMathLibrary.VSize` (`self.GetVelocity`)) 400.0)
      (`ActorComponent.Activate` (`self.VFX_footstepTrail`) false)
      (goto _label_2))))

(event `UpdateVisibilityState`
  (bind _overlappingactors (`PrimitiveComponent.GetOverlappingActors` (`self.CapsuleComponent`) null))
  ;[0.06511 0.1006 0.1177] Update the visibility according to the current zone
  (`|ExecutionSequence`
    (:`then_0`
      (set `self.IsHidden` true)
      (if (> (`KismetArrayLibrary.Array_Length` _overlappingactors) 0)
        (for _array_element _overlappingactors
          (cast `/Game/Blueprints/BP_Light` _array_element)
          (set `self.IsHidden` false)
          (break))))
    (:`then_1`
      (`self.OnPlayerVisibilityChanged`)
      (`self.ChangeAmbiance`))))

(event `ChangeAmbiance`
  ;[0.06511 0.1006 0.1177] Change the ambiance according to the zone
  (if (`self.IsHidden`)
    (bind (_direction _beta) (`Timeline|TimelineBeta` :!label _label_4)
      (:`Update`
        (`KismetMaterialLibrary.SetScalarParameterValue` "/Game/Materials/postProcess/MPC_PostProcess.MPC_PostProcess" "Beta" _beta)))
    (else
      (goto _label_4 :!via `Reverse`))))

(event `EndNight`
  ;[0.06511 0.1006 0.1177] Management of nights
  (`/Engine/EditorBlueprintResources/StandardMacros.IncrementInt` (`self.NightCount`)
    (:`  `
      (bind _asbp_top_down_game_instance (cast `/Game/Blueprints/System/BP_GameInstance` (`GameplayStatics.GetGameInstance`)))
      (`/Game/Blueprints/System/BP_GameInstance.DisplayEndScreen` _asbp_top_down_game_instance))))

(fn `ChangeCountdown`
  (if (== (`self.CountdownSeconds`) 0)
    (if (== (`self.CountdownMinutes`) 0)
      (if (not (`self.End`))
        (set `self.End` true)
        (`self.EndNight`))
      (else
        (`/Engine/EditorBlueprintResources/StandardMacros.DecrementInt` (`self.CountdownMinutes`)
          (:`  `
            (set `self.CountdownSeconds` 59)))))
    (else
      (`/Engine/EditorBlueprintResources/StandardMacros.DecrementInt` (`self.CountdownSeconds`)))))

(fn `InteractBehaviour`
  (locals (ClosestElementDistance :type "Float (double-precision)"))
  (bind _overlappingactors (`self.GetOverlappingActors` null))
  (set `self.ElementToInteract` null)
  (if (!= (`KismetArrayLibrary.Array_Length` _overlappingactors) 0)
    ;[0.06511 0.1006 0.1177] Finds the closest element to interact with
    (set `local.ClosestElementDistance` 10000.0)
    (for _array_element _overlappingactors
      (bind _asbpi_interact (cast `/Game/Blueprints/BPI_Interact` _array_element))
      (bind _isinteractable (`/Game/Blueprints/BPI_Interact.IsInteractable` _asbpi_interact))
      (if (and _isinteractable (< (`KismetMathLibrary.Vector_Distance` (`self.K2_GetActorLocation` _array_element) (`self.K2_GetActorLocation`)) (`local.ClosestElementDistance`)))
        (set `self.ElementToInteract` _asbpi_interact)))
    (cast `Actor` (`self.ElementToInteract`))
    (`self.DisableInput` (`GameplayStatics.GetPlayerController` 0))
    (bind _asbp_civil (cast `/Game/Blueprints/NPC/Civil/BP_Civil` (`self.ElementToInteract`))
      (:`then`
        (`CharacterMovementComponent.DisableMovement` (`Character.CharacterMovement` _asbp_civil)))
      (:`CastFailed`
        _))
    (bind _delay (`/Game/Blueprints/BPI_Interact.GetInteractionDelay` (`self.ElementToInteract`)))
    (bind _returnvalue (`KismetSystemLibrary.K2_SetTimerDelegate` (`|CreateDelegate` :!event `Interaction`) _delay))
    (set `self.CurrentInteractionTimer` _returnvalue)
    (`/Game/Blueprints/BPI_Interact.StartTimer` (`self.ElementToInteract`))))

(fn `UserConstructionScript`)