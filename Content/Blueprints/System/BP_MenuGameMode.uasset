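; BP_MenuGameMode is the menu's game mode, which shows the mouse cursor and runs a simulated clock.
; On BeginPlay it seeds CurrentHour from BeginningHour and starts a looping timer that calls UpdateCurrentHour every ten seconds.
; Each tick advances the minute stored in Y, carries into the hour in X on a twelve-hour wrap, and broadcasts the result through OnHourUpdated.
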(event `self.ReceiveBeginPlay`
  ;[0.06511 0.1006 0.1177] Initialization
  (set `PlayerController.bShowMouseCursor` true (`GameplayStatics.GetPlayerController` 0))
  (set `self.CurrentHour` (`self.BeginningHour`))
  (`KismetSystemLibrary.K2_SetTimer` null "UpdateCurrentHour" 10.0 true))

(fn `UpdateCurrentHour`
  (bind (_currenthour_x _currenthour_y) (`KismetMathLibrary.BreakVector2D` (`self.CurrentHour`)))
  (bind _returnvalue (+ _currenthour_y 1.0))
  (bind _returnvalue_2 (+ _currenthour_x 1.0))
  (bind _returnvalue_3 (>= _returnvalue 60.0))
  (bind _output_get (set `self.CurrentHour` (`KismetMathLibrary.MakeVector2D` (`KismetMathLibrary.SelectFloat` (`KismetMathLibrary.SelectFloat` _returnvalue_2 0.0 (< _returnvalue_2 12.0)) _currenthour_x _returnvalue_3) (`KismetMathLibrary.SelectFloat` 0.0 _returnvalue _returnvalue_3))))
  (`self.OnHourUpdated` _output_get))

(fn `UserConstructionScript`)